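; BP_gameIns is a game instance that holds a BP_saveGame object for score and high score data.
; On Init it loads that object from a slot and keeps it if the cast succeeds.
; Save replaces it with a newly created save object, zeroes Point and copies Point to HIScore when at least as high.
; Save never writes to a slot, and nothing in this file calls it.
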(event `self.ReceiveInit`
  (`self.LoadGame`))

(fn `LoadGame`
  (locals (NewLocalVar :type String))
  (bind _returnvalue (`GameplayStatics.LoadGameFromSlot` (`self.Slot`)))
  (bind _asbp_save_game (cast `/Game/SaveGame/BP_saveGame` _returnvalue))
  (set `self.BPSave` _asbp_save_game))

(fn `Save`
  (bind _bpsave (`self.BPSave`))
  (bind _returnvalue (`GameplayStatics.CreateSaveGameObject` "/Game/SaveGame/BP_saveGame.BP_saveGame_C"))
  (bind _output_get (set `self.BPSave` _returnvalue))
  (set `/Game/SaveGame/BP_saveGame.Point` 0 _output_get)
  (if (>= (`/Game/SaveGame/BP_saveGame.Point` _output_get) (`/Game/SaveGame/BP_saveGame.HIScore` _output_get))
    (set `/Game/SaveGame/BP_saveGame.HIScore` (`/Game/SaveGame/BP_saveGame.Point` _bpsave) _bpsave)))